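; SaveGameActor is a checkpoint-style trigger actor that saves a transform when anything begins overlapping its Box.
; It loads the "Save" slot, or creates a new BP_SaveGame if none exists.
; It then stores the Arrow component's world location and rotation at unit scale as the Transform and writes the slot back.
; The overlap is not filtered by actor, and this file only writes the transform, never applies it.
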(event OnComponentBeginOverlap(Box)
  (params (OverlappedComponent :type Primitive%20Component%20Object%20Reference) (OtherActor :type Actor%20Object%20Reference) (OtherComp :type Primitive%20Component%20Object%20Reference) (OtherBodyIndex :type Integer) (bFromSweep :type Boolean) (SweepResult :type Hit%20Result%20Structure%20%28by%20ref%29))
  (bind _arrow (Variables|Default|GetArrow))
  (bind _returnvalue (Transformation|GetWorldRotation _arrow))
  (bind _returnvalue_2 (Transformation|GetWorldLocation _arrow))
  (bind _returnvalue_3 (Math|Transform|MakeTransform _returnvalue_2 _returnvalue))
  (bind _returnvalue_4 (SaveGame|DoesSaveGameExist "Save"))
  (if _returnvalue_4
    (bind _returnvalue_5 (SaveGame|LoadGamefromSlot "Save"))
    (bind _output_get (Variables|Default|SetSaveGameSubClass _returnvalue_5))
    (bind _asbp_save_game (Utilities|Casting|CastToBP_SaveGame _output_get))
    (Variables|/Game/Blueprints/Save_Load_System/BP_SaveGame.BP_SaveGame_C|SetTransform _asbp_save_game _returnvalue_3)
    (SaveGame|SaveGametoSlot (Variables|Default|GetSaveGameSubClass) "Save")
    (else
      (bind _returnvalue_6 (SaveGame|CreateSaveGameObject "/Game/Blueprints/Save_Load_System/BP_SaveGame.BP_SaveGame_C"))
      (bind _output_get_2 (Variables|Default|SetSaveGameSubClass _returnvalue_6))
      (bind _asbp_save_game_2 (Utilities|Casting|CastToBP_SaveGame _output_get_2))
      (Variables|/Game/Blueprints/Save_Load_System/BP_SaveGame.BP_SaveGame_C|SetTransform _asbp_save_game_2 _returnvalue_3)
      (SaveGame|SaveGametoSlot (Variables|Default|GetSaveGameSubClass) "Save"))))

(fn ConstructionScript)