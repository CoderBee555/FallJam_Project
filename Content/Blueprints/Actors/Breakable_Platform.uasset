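; Breakable platform actor that vanishes shortly after the first-person character steps on it, then returns.
; A Box trigger overlap with FirstPersonCharacter waits BreakDuration, then disables the Cube's collision and hides it.
; After ReplenishDuration it restores the Cube's collision and visibility, so the platform can break again.
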(event OnComponentBeginOverlap(Box)
  (params (OverlappedComponent :type Primitive%20Component%20Object%20Reference) (OtherActor :type Actor%20Object%20Reference) (OtherComp :type Primitive%20Component%20Object%20Reference) (OtherBodyIndex :type Integer) (bFromSweep :type Boolean) (SweepResult :type Hit%20Result%20Structure%20%28by%20ref%29))
  (Utilities|Casting|CastToFirstPersonCharacter OtherActor)
  (Utilities|FlowControl|Delay (Variables|Default|GetBreak%20Duration))
  (Collision|SetCollisionEnabled (Variables|Default|GetCube) "NoCollision")
  (Rendering|SetVisibility (Variables|Default|GetCube) false false)
  (Utilities|FlowControl|Delay (Variables|Default|GetReplenish%20Duration))
  (Collision|SetCollisionEnabled (Variables|Default|GetCube) "QueryAndPhysics")
  (Rendering|SetVisibility (Variables|Default|GetCube) true false))

(event Collision|EventActorBeginOverlap
  (params (OtherActor :type Actor%20Object%20Reference)))

(event EventTick
  (params (DeltaSeconds :type Float%20%28single-precision%29)))

(event EventBeginPlay)

(fn ConstructionScript)