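; Parkour component that gives a character side wall runs, forward wall climbs, and jump-offs that feed the FirstPersonCharacter combo.
; A looping timer traces right, left and forward while falling, propelling the character with LaunchCharacter and easing gravity toward a wall-run value.
; Ending a run restores gravity and briefly suppresses detection, while the stored jump-off normal blocks same-facing walls until landing resets it.
; Tick rolls the camera during side runs.
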(event Custom|Initialize
  (params (Character :type Character%20Object%20Reference))
  (bind _output_get (Variables|Default|SetCharacter Character))
  (bind _output_get_2 (Variables|Default|SetCharacter%20Movement (Variables|/Script/Engine.Character|GetCharacterMovement _output_get)))
  (Variables|Default|SetDefault%20Gravity (Variables|/Script/Engine.CharacterMovementComponent|GetGravityScale _output_get_2))
  (Utilities|Time|SetTimerbyEvent (delegate Custom|WallRunUpdateEvent) 0.02 true))

(event Custom|Land%20Event
  (CallFunction|WallRunEnd 0.0)
  (Variables|Default|SetWallRunSuppressed? false)
  (Variables|Default|SetWallRunUpDoOnce true)
  (Variables|Default|SetLast%20Wall%20Normal "10.000000, 0, 0"))

(event Custom|Jump%20Event
  (CallFunction|WallRunJump))

(event Custom|WallRunUpdateEvent
  (if (not (Variables|Default|GetWallRunSuppressed?))
    (CallFunction|WallRunUpdate)))

(event Custom|ResetWallRunSuppression
  (Utilities|Time|ClearTimerbyFunctionName 0 "ResetWallRunSuppression")
  (Variables|Default|SetWallRunSuppressed? false))

(event EventTick
  (params (DeltaSeconds :type Float%20%28single-precision%29))
  (CallFunction|CameraTick))

(fn WallRunUpdate
  (bind _on_wall (CallFunction|WallRunMovement (Transformation|GetActorLocation (Variables|Default|GetCharacter)) (.Right (Utilities|WallRunEndVectors)) -1.0 false))
  (if _on_wall
    (Variables|Default|SetWallRunning true)
    (Variables|Default|SetWallRunningR true)
    (Variables|Default|SetWallRunningL false)
    (Variables|Default|SetWallRunningUP false)
    (Variables|/Script/Engine.CharacterMovementComponent|SetGravityScale (Variables|Default|GetCharacter%20Movement) (Math|Interpolation|FInterpTo (Variables|/Script/Engine.CharacterMovementComponent|GetGravityScale (Variables|Default|GetCharacter%20Movement)) (Variables|Default|GetWallRunTargetGravity) (Utilities|Time|GetWorldDeltaSeconds) 1e+01) :!label _label)
    (elif (Variables|Default|GetWallRunningR)
      (CallFunction|WallRunEnd 1.0)
      (Variables|Default|SetWallRunUpDoOnce true)
      (else
        (bind _on_wall_2 (CallFunction|WallRunMovement (Transformation|GetActorLocation (Variables|Default|GetCharacter)) (.Left (Utilities|WallRunEndVectors)) 1.0 false))
        (if _on_wall_2
          (Variables|Default|SetWallRunning true)
          (Variables|Default|SetWallRunningR false)
          (Variables|Default|SetWallRunningL true)
          (Variables|Default|SetWallRunningUP false)
          (goto _label)
          (elif (Variables|Default|GetWallRunningL)
            (CallFunction|WallRunEnd 1.0)
            (elif (Variables|Default|GetWallRunUpDoOnce)
              (bind _on_wall_3 (CallFunction|WallRunMovement (Transformation|GetActorLocation (Variables|Default|GetCharacter)) (.Up (Utilities|WallRunEndVectors)) 1.0 true))
              (if _on_wall_3
                (Variables|Default|SetWallRunning true)
                (Variables|Default|SetWallRunningR false)
                (Variables|Default|SetWallRunningL false)
                (Variables|Default|SetWallRunningUP true)
                (Variables|Default|SetWallRunUpDoOnce false)
                (goto _label)
                (else
                  (CallFunction|WallRunEnd 1.0))))))))))

(fn WallRunMovement
  (params (Start :type Vector) (End :type Vector) (WallRunDirection :type Float%20%28single-precision%29) (WallRunUp? :type Boolean))
  (bind _outhit (Collision|LineTraceByChannel Start End "TraceTypeQuery1" false 0 "None"))
  (if (.bBlockingHit (Collision|BreakHitResult _outhit))
    (if (and (AI|Components|NavMovement|IsFalling (Variables|Default|GetCharacter%20Movement)) (.ReturnValue (Utilities|ValidWallRunVector? (.Normal (Collision|BreakHitResult _outhit)))))
      (if (Math|Vector|Equal(Vector) (.OutVector (Utilities|ValidWallRunVector? (.Normal (Collision|BreakHitResult _outhit)))) (Variables|Default|GetLast%20Wall%20Normal) 0.0001)
        (return false)
        (else
          (Variables|Default|SetWall%20Run%20Normal (.OutVector (Utilities|ValidWallRunVector? (.Normal (Collision|BreakHitResult _outhit)))))
          (Character|LaunchCharacter (Variables|Default|GetCharacter) (Utilities|PlayertoWallVector) false false)
          (if WallRunUp?
            (Character|LaunchCharacter (Variables|Default|GetCharacter) (Math|Vector|MakeVector 0.0 0.0 7e+02) false true)
            (return true)
            (else
              (Character|LaunchCharacter (Variables|Default|GetCharacter) (* (Math|Vector|CrossProduct (Variables|Default|GetWall%20Run%20Normal) "0, 0,1.000000") (* WallRunDirection (Variables|Default|GetWallRunSpeed))) true false)
              (return true)))))
      (else
        (return false)))
    (else
      (return false))))

(fn WallRunEnd
  (params (Reset%20Time :type Float%20%28single-precision%29))
  (if (Variables|Default|GetWallRunning)
    (Variables|Default|SetWallRunningL false)
    (Variables|Default|SetWallRunningR false)
    (Variables|Default|SetWallRunning false)
    (Variables|Default|SetWallRunningUP false)
    (Variables|/Script/Engine.CharacterMovementComponent|SetGravityScale (Variables|Default|GetCharacter%20Movement) (Variables|Default|GetDefault%20Gravity))
    (CallFunction|SuppressWallRun Reset%20Time)))

(fn SuppressWallRun
  (params (Delay :type Float%20%28single-precision%29))
  (Variables|Default|SetWallRunSuppressed? true)
  (Utilities|Time|SetTimerbyFunctionName 0 "ResetWallRunSuppression" Delay))

(fn CameraTick
  (if (Variables|Default|GetWallRunningL)
    (CallFunction|CameraTilt 15.0)
    (elif (Variables|Default|GetWallRunningR)
      (CallFunction|CameraTilt -15.0)
      (else
        (CallFunction|CameraTilt 0.0)))))

(fn CameraTilt
  (params (Target%20x%20%28Roll%29 :type Float%20%28single-precision%29))
  (bind _character (Variables|Default|GetCharacter))
  (bind _returnvalue (Pawn|GetController _character))
  (bind _returnvalue_2 (Pawn|GetControlRotation _returnvalue :!class /Script/Engine.Controller))
  (bind (_roll _pitch _yaw) (Math|Rotator|BreakRotator _returnvalue_2))
  (Pawn|SetControlRotation (Pawn|GetController (Variables|Default|GetCharacter)) (Math|Interpolation|RInterpTo _returnvalue_2 (Math|Rotator|MakeRotator Target%20x%20%28Roll%29 _pitch _yaw) (Utilities|Time|GetWorldDeltaSeconds) 1e+01)))

(fn WallRunJump
  (bind _wall_run_normal (Variables|Default|GetWall%20Run%20Normal))
  (bind (_x _y) (Math|Vector|BreakVector _wall_run_normal))
  (if (Variables|Default|GetWallRunning)
    (CallFunction|WallRunEnd 0.35)
    (Character|LaunchCharacter (Variables|Default|GetCharacter) (Math|Vector|MakeVector (* (Variables|Default|GetWall%20Run%20Jump%20Off%20Force) _x) (* _y (Variables|Default|GetWall%20Run%20Jump%20Off%20Force)) (Variables|Default|GetWall%20Run%20Jump%20Height)) false true)
    (bind _asfirst_person_character (Utilities|Casting|CastToFirstPersonCharacter (Variables|Default|GetCharacter)))
    (Default|AddCombo _asfirst_person_character (Variables|/Game/FirstPersonBP/Blueprints/FirstPersonCharacter.FirstPersonCharacter_C|GetCanAddCombo _asfirst_person_character))
    (Variables|Default|SetLast%20Wall%20Normal (Variables|Default|GetWall%20Run%20Normal))))